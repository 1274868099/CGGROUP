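; BP_Random is a rock spawner that launches batches of randomly scaled Rock_Blueprint actors along world +X.
; A custom event starts on BeginPlay and re-arms itself with a three-second timer, spawning a batch sized by 生成数量 each time.
; Rocks spawn at random points around the Box and receive a mass-independent impulse.
; The construction script sizes the Box from 生成的范围大小, but spawning uses a hardcoded half-size instead.
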(event Custom|自定义事件
  (bind _returnvalue (Math|Random|RandomFloatinRange 0.4 0.7))
  (Utilities|Time|SetTimerbyEvent (delegate Custom|自定义事件) 3.0)
  (for _index (range 0 (Variables|Default|Get生成数量))
    (bind _returnvalue_2 (Game|SpawnActorfromClass "/Game/_Game/BP/BluePrintClasses/Rock_Blueprint.Rock_Blueprint_C" (Math|Transform|MakeTransform (Math|Random|RandomPointinBoundingBox (Transformation|GetWorldLocation (Variables|Default|GetBox)) "150.000000,800.000000,800.000000") "0, 0, 0" (Math|Vector|MakeVector _returnvalue _returnvalue _returnvalue)) "Undefined" 0 0))
    (Physics|AddImpulse (Variables|/Script/Engine.StaticMeshActor|GetStaticMeshComponent _returnvalue_2) "100.000000,0.000000,0.000000" "None" true)))

(event EventBeginPlay
  (CallFunction|自定义事件))

(fn ConstructionScript
  (Components|Box|SetBoxExtent (Variables|Default|GetBox) (Variables|Default|Get生成的范围大小) true))
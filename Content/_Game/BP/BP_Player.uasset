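; BP_Player is the player actor, which fires bullets and takes damage.
; Left mouse clicks spawn BP_Bullet at two Arrow components through separate input events.
; Any Box overlap or the H key calls ApplyDamage, which subtracts Damage from clamped Health and prints it.
; Health is checked before subtraction, so the actor is destroyed on the call after it reaches zero.
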(event OnComponentBeginOverlap(Box)
  (params (OverlappedComponent :type Primitive%20Component%20Object%20Reference) (OtherActor :type Actor%20Object%20Reference) (OtherComp :type Primitive%20Component%20Object%20Reference) (OtherBodyIndex :type Integer) (bFromSweep :type Boolean) (SweepResult :type Hit%20Result%20Structure%20%28by%20ref%29))
  (CallFunction|ApplyDamage))

(event EventBeginPlay
  (bind _output_get (Variables|Default|SetMaxHealth 1e+02))
  (Variables|Default|SetHealth _output_get))

(event EventTick
  (params (DeltaSeconds :type Float%20%28single-precision%29)))

(event Input|MouseEvents|LeftMouseButton
  (params (Key :type Key%20Structure :default "None"))
  (bind _arrow2 (Variables|Default|GetArrow2))
  (bind _returnvalue (Transformation|GetWorldTransform _arrow2))
  (:Pressed
    (Game|SpawnActorfromClass "/Game/_Game/BP/BP_Bullet.BP_Bullet_C" (Math|Transform|MakeTransform (.location _returnvalue) (.rotation _returnvalue) "1.000000,1.000000,1.000000") "AlwaysSpawn" 0 0)))

(event Input|MouseEvents|LeftMouseButton
  (params (Key :type Key%20Structure :default "None"))
  (bind _arrow1 (Variables|Default|GetArrow1))
  (bind _returnvalue (Transformation|GetWorldTransform _arrow1))
  (:Pressed
    (Game|SpawnActorfromClass "/Game/_Game/BP/BP_Bullet.BP_Bullet_C" (Math|Transform|MakeTransform (.location _returnvalue) (.rotation _returnvalue) "1.000000,1.000000,1.000000") "AlwaysSpawn" 0 0)))

(event Input|KeyboardEvents|H
  (params (Key :type Key%20Structure :default "None"))
  (:Pressed
    (CallFunction|ApplyDamage)))

(fn ConstructionScript)

(fn ApplyDamage
  (if (<= (Variables|Default|GetHealth) 0.0)
    (Actor|DestroyActor)
    (else
      (bind _output_get (Variables|Default|SetHealth (Math|Float|Clamp(Float) (- (Variables|Default|GetHealth) (Variables|Default|GetDamage)) 0.0 (Variables|Default|GetMaxHealth))))
      (Development|PrintString (Utilities|String|ToString(Float) _output_get)))))